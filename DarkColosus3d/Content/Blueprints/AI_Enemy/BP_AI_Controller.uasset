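; BP_AI_Controller is an enemy AI controller that detects a target by sight and passes it to a behavior tree for chasing.
; It starts BT_Basic on BeginPlay.
; AIPerception updates write the sensed actor to the TargetActor blackboard key on successful sight.
; Lost sight, or any non-sight stimulus, clears that key, even if another target was set.
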(event OnTargetPerceptionUpdated(AIPerception)
  (params (Actor :type Actor%20Object%20Reference) (Stimulus :type AI%20Stimulus%20Structure))
  ;[1 1 1] Detect and Chase Target
  (bind _returnvalue (Class|AIPerceptionSystem|GetSenseClassforStimulus Stimulus))
  (if (== _returnvalue "/Script/AIModule.AISense_Sight")
    (if (.bSuccessfullySensed (Utilities|Struct|BreakAIStimulus Stimulus))
      (AI|Components|Blackboard|SetValueasObject (AI|GetBlackboard 0) (Utilities|Name|MakeLiteralName "TargetActor") Actor)
      (else
        (AI|Components|Blackboard|SetValueasObject (AI|GetBlackboard 0) (Utilities|Name|MakeLiteralName "TargetActor") 0 :!label _label)))
    (else
      (goto _label))))

(event EventBeginPlay
  (AI|RunBehaviorTree "/Game/Blueprints/AI_Enemy/BT_Basic.BT_Basic"))

(event EventTick
  (params (DeltaSeconds :type Float%20%28single-precision%29)))

(fn ConstructionScript)