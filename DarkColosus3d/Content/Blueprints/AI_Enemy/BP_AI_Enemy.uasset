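; Enemy AI character that chases the player once seen and provides hit-reaction and death events.
; PawnSensing sets a seeing flag, never cleared here, and triggers an AI move toward player 0 without checking which pawn was seen.
; Health starts at max; the death event destroys the actor at exactly zero, but nothing here applies damage.
; The hit-detect function is an empty stub with an unconnected sphere trace.
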(event OnSeePawn(PawnSensing)
  (params (Pawn :type Pawn%20Object%20Reference))
  (Variables|Default|SetisPawnSeeing? true)
  (CallFunction|FollowPlayer))

(event Custom|AI%20Died
  ;[1 1 1] AI Died
  (if (== (Variables|Default|GetCurrentHealth) 0.0)
    (Actor|DestroyActor)))

(event Custom|AI%20Hit%20Reaction
  (Animation|PlayAnimMontage "/Game/Blueprints/Animations/AM_Hit_reaction.AM_Hit_reaction" 1.0 "01"))

(event Custom|FollowPlayer
  (if (Variables|Default|GetisPawnSeeing?)
    (AI|AIMoveTo self "0, 0, 0" (Game|GetPlayerCharacter 0) 5.0 false)))

(event EventBeginPlay
  (|CallParentFunction)
  (Variables|Default|SetCurrentHealth (Variables|Default|GetMaxHealth)))

(event Collision|EventActorBeginOverlap
  (params (OtherActor :type Actor%20Object%20Reference)))

(event EventTick
  (params (DeltaSeconds :type Float%20%28single-precision%29)))

(fn ConstructionScript
  (|CallParentFunction))

(fn AIHitDetect)